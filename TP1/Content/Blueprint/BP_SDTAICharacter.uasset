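; BP_SDTAICharacter is an AI character Blueprint that shows its pickup and death counts as an on-screen debug readout.
; Each Tick it prints the actor name with NbPickup and NbDeath as a screen string lasting one frame, without logging it.
; Its BeginPlay, overlap and construction script are empty, and this Blueprint only reads the counters, never changing them.
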(event `self.ReceiveBeginPlay`)

(event `self.ReceiveActorBeginOverlap`
  (params (OtherActor :type "Actor Object Reference")))

(event `self.ReceiveTick`
  (params (DeltaSeconds :type "Float (single-precision)"))
  (`KismetSystemLibrary.PrintString` (`KismetStringLibrary.Concat_StrStr` (`KismetSystemLibrary.GetObjectName` self) (`KismetTextLibrary.Conv_TextToString` (`KismetTextLibrary.Conv_StringToText` " - nb_pickup : ")) (`KismetStringLibrary.Conv_IntToString` (`self.nb_pickup`)) (`KismetTextLibrary.Conv_TextToString` (`KismetTextLibrary.Conv_StringToText` " nb_death : ")) (`KismetStringLibrary.Conv_IntToString` (`self.nb_death`))) true false (struct :`R` 0.744792 :`B` 0.589951 :`A` 1.0) DeltaSeconds))

(fn `UserConstructionScript`)